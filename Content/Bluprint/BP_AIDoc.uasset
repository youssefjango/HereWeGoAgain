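; Doctor AI actor that walks to the hospital player on BeginPlay and triggers a dialog that ends in a level change.
; On arrival it plays a line at its own location and a louder, higher-pitched dialog sound for each "SoundPatient"-tagged actor.
; Those sounds spawn at the tagged actor's rotation X vector, not its location.
; When a dialog sound finishes, the MainHall level opens.
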(event `self.ReceiveBeginPlay`
  (bind _asbp_hospital_player (cast `/Game/Bluprint/BP_HospitalPlayer` (`GameplayStatics.GetPlayerPawn` 0)))
  (`|AIMoveTo` null (0.0 0.0 0.0) _asbp_hospital_player 150.0
    (:`OnSuccess`
      (`GameplayStatics.SpawnSoundAtLocation` "/Game/Assets/Musics/Dialog/Line_1.Line_1" (`self.K2_GetActorLocation`) (struct) 1.0 1.0 0.0 null null)
      (bind _outactors (`GameplayStatics.GetAllActorsWithTag` "SoundPatient"))
      (for _array_element _outactors
        (bind _returnvalue (`GameplayStatics.SpawnSoundAtLocation` "/Game/Assets/Musics/Dialog/DialogSound.DialogSound" (`KismetMathLibrary.Conv_RotatorToVector` (`self.K2_GetActorRotation` _array_element)) (struct) 3.0 1.3 0.0 null null))
        (add `AudioComponent.OnAudioFinished` _returnvalue (delegate `OpenLevel`))))))

(event `OpenLevel`
  (`GameplayStatics.OpenLevel` "MainHall"))

(fn `UserConstructionScript`)