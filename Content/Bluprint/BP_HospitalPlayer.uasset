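; Player pawn for a hospital scene, offering mouse look within a restricted view arc and a periodic blinking effect.
; BeginPlay adds the mouse-look Enhanced Input context, clamps camera manager pitch and yaw, and starts a looping blink timer.
; Each blink replays a timeline whose single track drives both eye roughness and openness in the MPC_Blink material parameter collection.
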(event `Blink`
  (bind (_direction _newtrack_0) (`Timeline|TL_Blink` :!via `PlayFromStart`)
    (:`Update`
      (`KismetMaterialLibrary.SetScalarParameterValue` "/Game/Assets/Hospital/MPC_Blink.MPC_Blink" "EyeRoughness" _newtrack_0)
      (`KismetMaterialLibrary.SetScalarParameterValue` "/Game/Assets/Hospital/MPC_Blink.MPC_Blink" "AmountOpened" _newtrack_0))))

(event `self.ReceiveBeginPlay`
  (bind _returnvalue (`GameplayStatics.GetPlayerCameraManager` 0))
  (bind _returnvalue_2 (pcsubsystem `EnhancedInputLocalPlayerSubsystem` (`GameplayStatics.GetPlayerController` 0)))
  (`|ExecutionSequence`
    (:`then_0`
      (`/Engine/EditorBlueprintResources/StandardMacros.IsValid` _returnvalue_2
        (:`Is Valid`
          (`EnhancedInputSubsystemInterface.AddMappingContext` _returnvalue_2 "/Game/Input/IMC_MouseLook.IMC_MouseLook" 0 (struct)))))
    (:`then_1`
      (set `PlayerCameraManager.ViewPitchMax` 90.0 _returnvalue)
      (set `PlayerCameraManager.ViewPitchMin` -30.0 _returnvalue)
      (set `PlayerCameraManager.ViewYawMin` 120.0 _returnvalue)
      (set `PlayerCameraManager.ViewYawMax` 220.0 _returnvalue))
    (:`then_2`
      (`KismetSystemLibrary.K2_SetTimerDelegate` (delegate `Blink`) 2.0 true))))

(event `EnhancedInput|/Game/Input/Actions/IA_MouseLook`
  (params (ActionValue :type "Vector2D Structure") (ElapsedSeconds :type "Float (double-precision)") (TriggeredSeconds :type "Float (double-precision)") (InputAction :type "InputAction Object Reference" :default "/Game/Input/Actions/IA_MouseLook.IA_MouseLook"))
  (bind (_x _y) (`KismetMathLibrary.BreakVector2D` ActionValue))
  (:`Triggered`
    (`self.AddControllerYawInput` _x)
    (`self.AddControllerPitchInput` _y)))

(fn `UserConstructionScript`)