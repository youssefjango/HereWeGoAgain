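; BP_Tree is a harvestable tree actor that yields wood to the player when chopped down.
; Each TakeHit call removes one point of TreeHealth; at zero it calls AddWood on the player's BP_RogueCharacter and destroys itself.
; An IsDestroyed flag guards against further hits, and a failed character cast leaves the tree standing.
; The construction script applies the TreeStaticMesh variable to the mesh component.
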(event `TakeHit`
  (if (not (`self.isDestroyed`))
    (set `self.TreeHealth` (- (`self.TreeHealth`) 1.0))
    (if (<= (`self.TreeHealth`) 0.0)
      (bind _asbp_rogue_character (cast `/Game/RogueCharacter/Demo/ThirdPerson/Blueprints/BP_RogueCharacter` (`GameplayStatics.GetPlayerPawn` 0)))
      (`/Game/RogueCharacter/Demo/ThirdPerson/Blueprints/BP_RogueCharacter.AddWood` _asbp_rogue_character 0)
      (`self.DestroyTree`))))

(event `DestroyTree`
  (set `self.isDestroyed` true)
  (`self.K2_DestroyActor`))

(fn `UserConstructionScript`
  (`StaticMeshComponent.SetStaticMesh` (`self.TreeSMesh`) (`self.TreeStaticMesh`)))