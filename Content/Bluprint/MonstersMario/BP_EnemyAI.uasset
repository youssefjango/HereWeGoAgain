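; BP_EnemyAI is an AI enemy that detects and attacks the rogue player character.
; Pawn sensing sets HasSeenPlayer on its controller's Blackboard.
; AttackPlayer sphere-traces for pawns around a point just ahead, then plays a sound and montage and applies damage if the hit is the player.
; DamageHealth subtracts health and, at zero, reports the death to MarioGM before destroying the actor.
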(event `self.PawnSensing.OnSeePawn`
  (params (Pawn :type "Pawn Object Reference"))
  (cast `/Game/RogueCharacter/Demo/ThirdPerson/Blueprints/BP_RogueCharacter` Pawn)
  (`BlackboardComponent.SetValueAsBool` (`AIBlueprintHelperLibrary.GetBlackboard` (`AIBlueprintHelperLibrary.GetAIController` self)) "HasSeenPlayer" true))

(event `AttackPlayer`
  (bind _returnvalue (`self.K2_GetActorLocation`))
  (bind (_outhit _returnvalue_2) (`KismetSystemLibrary.SphereTraceSingleForObjects` _returnvalue (+ (* (`KismetMathLibrary.GetForwardVector` (`self.K2_GetActorRotation`)) 50.0) _returnvalue) 300.0 (`|MakeArray` "ObjectTypeQuery3" :!type "EObjectTypeQuery Enum")))
  (if _returnvalue_2
    (bind (_bblockinghit _binitialoverlap _time _distance _location _impactpoint _normal _impactnormal _physmat _hitactor) (`GameplayStatics.BreakHitResult` _outhit))
    (cast `/Game/RogueCharacter/Demo/ThirdPerson/Blueprints/BP_RogueCharacter` _hitactor)
    (`GameplayStatics.PlaySoundAtLocation` "/Game/Assets/Musics/Mario_Mob.Mario_Mob" (`self.K2_GetActorLocation`) (struct) 1.0 1.0 0.0 null null null null)
    (`self.PlayAnimMontage` (`self.AnimMontageAttack`))
    (`GameplayStatics.ApplyDamage` _hitactor (`self.AttackDamage`))))

(fn `DamageHealth`
  (params (DamageVal :type "Float (double-precision)"))
  (bind _output_get (set `self.Health` (- (`self.Health`) DamageVal)))
  (if (<= _output_get 0.0)
    (bind _asmario_gm (cast `/Game/Bluprint/GameModes/MarioGM` (`GameplayStatics.GetGameMode`)))
    (`/Game/Bluprint/GameModes/MarioGM.IncrementEnemyDeath` _asmario_gm)
    (`self.K2_DestroyActor`)))

(fn `UserConstructionScript`)